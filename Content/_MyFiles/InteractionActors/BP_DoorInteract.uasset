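; BP_DoorInteract is an interactable door actor that toggles between a closed and an open position.
; On BeginPlay it records its current location as the closed position.
; Each BlueprintInteraction event flips IsOpen and instantly sets the actor's location to ClosedLocation or Openlocation, with no sweep or interpolation.
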(event `self.ReceiveBeginPlay`
  (set `self.ClosedLocation` (`self.K2_GetActorLocation` self)))

(event `self.blueprintInteraction`
  (params (Character :type "BaseCharacter Object Reference"))
  (if (`self.bIsOpen`)
    (`self.K2_SetActorLocation` (`self.ClosedLocation`))
    (set `self.bIsOpen` false)
    (else
      (`self.K2_SetActorLocation` (`self.Openlocation`))
      (set `self.bIsOpen` true))))

(fn `UserConstructionScript`)